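; BP_LoopPlatform is a moving platform that starts shuttling between StartLocation and EndLocation when something overlaps its Box.
; If PlatformBehavior is Loop, Timeline_0 lerps the mesh's relative location, playing or reversing according to the Switcher flag.
; Each update flips Switcher on reaching either endpoint and re-enters the behavior check, creating a ping-pong loop without a separate timer or Finished event.
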(event OnComponentBeginOverlap(Box)
  (params (OverlappedComponent :type Primitive%20Component%20Object%20Reference) (OtherActor :type Actor%20Object%20Reference) (OtherComp :type Primitive%20Component%20Object%20Reference) (OtherBodyIndex :type Integer) (bFromSweep :type Boolean) (SweepResult :type Hit%20Result%20Structure%20%28by%20ref%29))
  (bind _platformmesh (Variables|Default|GetPlatformMesh))
  (bind _relativelocation (Variables|/Script/Engine.SceneComponent|GetRelativeLocation _platformmesh))
  ;[0.879 0.4271 1] Behaviour cheking
  (if (Utilities|Enum|Equal(Enum) (Variables|Default|GetPlatformBehavior) "Loop") :!label _label
    (if (Variables|Default|GetSwitcher)
      ;[1 0.8342 0.349] Platform moving
      (bind _newtrack_0 (Timeline|Timeline_0 Play)
        (:Update
          (Transformation|SetRelativeLocation (Variables|Default|GetPlatformMesh) (Math|Vector|Lerp(Vector) (Variables|Default|GetStartLocation) (Variables|Default|GetEndLocation) _newtrack_0) false false)
          ;[0.5781 0.6743 1] Looping Mechanic
          (if (Math|Vector|Equal(Vector) _relativelocation (Variables|Default|GetEndLocation) 0.0001)
            (Variables|Default|SetSwitcher false)
            (goto _label)
            (elif (Math|Vector|Equal(Vector) _relativelocation (Variables|Default|GetStartLocation) 0.0001)
              (Variables|Default|SetSwitcher true)
              (goto _label)
              (else
                (goto _label))))))
      (else
        (Timeline|Timeline_0 Reverse)))))

(fn ConstructionScript)